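; Blueprint function library of miscellaneous utilities for networking checks, mouse centering, vector clamping and UMG widget styling.
; Widget helpers swap progress bar fill or background images, image brushes and box width/height overrides, rebuilding style structs so other properties carry over.
; SetTextFontMaterial only returns a rebuilt font info without applying it to the target.
; The font and image brush helpers act only when the supplied asset is valid.
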(fn IsNetworked
  (return (not (Class|KismetSystemLibrary|IsStandalone))))

(fn CenterMousePosition
  (params (PlayerIndex :type Integer))
  (bind _returnvalue (Viewport|GetViewportSize))
  (bind (_x _y) (Math|Vector2D|BreakVector2D _returnvalue))
  (Class|PlayerController|SetMouseLocation (Game|GetPlayerController 0 PlayerIndex) (Math|Float|Truncate (/ _x 2.0)) (Math|Float|Truncate (/ _y 2.0))))

(fn SetFillImage
  (params (Target :type Progress%20Bar%20Object%20Reference) (FillImage :type Texture%202D%20Object%20Reference))
  (bind _output_get (Variables|/Script/UMG.ProgressBar|SetWidgetStyle Target (Utilities|Struct|MakeProgressBarStyle (.BackgroundImage (Utilities|Struct|BreakProgressBarStyle (Variables|/Script/UMG.ProgressBar|GetWidgetStyle Target))) (Utilities|Struct|MakeSlateBrush (.DrawAs (Utilities|Struct|BreakSlateBrush (.FillImage (Utilities|Struct|BreakProgressBarStyle (Variables|/Script/UMG.ProgressBar|GetWidgetStyle Target))))) (.Tiling (Utilities|Struct|BreakSlateBrush (.FillImage (Utilities|Struct|BreakProgressBarStyle (Variables|/Script/UMG.ProgressBar|GetWidgetStyle Target))))) (.Mirroring (Utilities|Struct|BreakSlateBrush (.FillImage (Utilities|Struct|BreakProgressBarStyle (Variables|/Script/UMG.ProgressBar|GetWidgetStyle Target))))) (.ImageSize (Utilities|Struct|BreakSlateBrush (.FillImage (Utilities|Struct|BreakProgressBarStyle (Variables|/Script/UMG.ProgressBar|GetWidgetStyle Target))))) (.Margin (Utilities|Struct|BreakSlateBrush (.FillImage (Utilities|Struct|BreakProgressBarStyle (Variables|/Script/UMG.ProgressBar|GetWidgetStyle Target))))) (.TintColor (Utilities|Struct|BreakSlateBrush (.FillImage (Utilities|Struct|BreakProgressBarStyle (Variables|/Script/UMG.ProgressBar|GetWidgetStyle Target))))) (.OutlineSettings (Utilities|Struct|BreakSlateBrush (.FillImage (Utilities|Struct|BreakProgressBarStyle (Variables|/Script/UMG.ProgressBar|GetWidgetStyle Target))))) FillImage) (.MarqueeImage (Utilities|Struct|BreakProgressBarStyle (Variables|/Script/UMG.ProgressBar|GetWidgetStyle Target))) (.EnableFillAnimation (Utilities|Struct|BreakProgressBarStyle (Variables|/Script/UMG.ProgressBar|GetWidgetStyle Target))))))
  (return _output_get))

(fn SetBackgroundImage
  (params (Target :type Progress%20Bar%20Object%20Reference) (BackgroundImage :type Texture%202D%20Object%20Reference))
  (bind _output_get (Variables|/Script/UMG.ProgressBar|SetWidgetStyle Target (Utilities|Struct|MakeProgressBarStyle (Utilities|Struct|MakeSlateBrush (.DrawAs (Utilities|Struct|BreakSlateBrush (.BackgroundImage (Utilities|Struct|BreakProgressBarStyle (Variables|/Script/UMG.ProgressBar|GetWidgetStyle Target))))) (.Tiling (Utilities|Struct|BreakSlateBrush (.BackgroundImage (Utilities|Struct|BreakProgressBarStyle (Variables|/Script/UMG.ProgressBar|GetWidgetStyle Target))))) (.Mirroring (Utilities|Struct|BreakSlateBrush (.BackgroundImage (Utilities|Struct|BreakProgressBarStyle (Variables|/Script/UMG.ProgressBar|GetWidgetStyle Target))))) (.ImageSize (Utilities|Struct|BreakSlateBrush (.BackgroundImage (Utilities|Struct|BreakProgressBarStyle (Variables|/Script/UMG.ProgressBar|GetWidgetStyle Target))))) (.Margin (Utilities|Struct|BreakSlateBrush (.BackgroundImage (Utilities|Struct|BreakProgressBarStyle (Variables|/Script/UMG.ProgressBar|GetWidgetStyle Target))))) (.TintColor (Utilities|Struct|BreakSlateBrush (.BackgroundImage (Utilities|Struct|BreakProgressBarStyle (Variables|/Script/UMG.ProgressBar|GetWidgetStyle Target))))) (.OutlineSettings (Utilities|Struct|BreakSlateBrush (.BackgroundImage (Utilities|Struct|BreakProgressBarStyle (Variables|/Script/UMG.ProgressBar|GetWidgetStyle Target))))) BackgroundImage) (.FillImage (Utilities|Struct|BreakProgressBarStyle (Variables|/Script/UMG.ProgressBar|GetWidgetStyle Target))) (.MarqueeImage (Utilities|Struct|BreakProgressBarStyle (Variables|/Script/UMG.ProgressBar|GetWidgetStyle Target))) (.EnableFillAnimation (Utilities|Struct|BreakProgressBarStyle (Variables|/Script/UMG.ProgressBar|GetWidgetStyle Target))))))
  (return _output_get))

(fn SetBoxSize
  (params (Target :type Size%20Box%20Object%20Reference) (Width :type Float%20%28single-precision%29) (Height :type Float%20%28single-precision%29))
  (Class|SizeBox|SetWidthOverride Target Width)
  (Class|SizeBox|SetHeightOverride Target Height))

(fn Clamp(Vector)
  (params (Value :type Vector) (Min :type Vector) (Max :type Vector))
  (return (Math|Vector|MakeVector (Math|Float|Clamp(Float) (.x Value) (.x Min) (.x Max)) (Math|Float|Clamp(Float) (.y Value) (.y Min) (.y Max)) (Math|Float|Clamp(Float) (.z Value) (.z Min) (.z Max)))))

(fn SetTextFontMaterial
  (params (Target :type Text%20Block%20Object%20Reference) (FontMaterial :type Object%20Object%20Reference))
  (bind _font (Variables|/Script/UMG.TextBlock|GetFont Target))
  (bind (_fontobject _fontmaterial _outlinesettings _typefacefontname _size _letterspacing _skewamount _bforcemonospaced _monospacedwidth) (Utilities|Struct|BreakSlateFontInfo _font))
  (Utilities|IsValid FontMaterial
    (:Is%20Valid
      (return (Utilities|Struct|MakeSlateFontInfo _fontobject FontMaterial _outlinesettings _typefacefontname _size _letterspacing _skewamount _bforcemonospaced _monospacedwidth)))))

(fn SetImageBrush
  (params (Target :type Image%20Object%20Reference) (ImageText :type Object%20Object%20Reference))
  (bind _brush (Variables|/Script/UMG.Image|GetBrush Target))
  (bind (_drawas _tiling _mirroring _imagesize _margin _tintcolor _outlinesettings) (Utilities|Struct|BreakSlateBrush _brush))
  (bind _slatebrush (Utilities|Struct|MakeSlateBrush _drawas _tiling _mirroring _imagesize _margin _tintcolor _outlinesettings ImageText))
  (Utilities|IsValid ImageText
    (:Is%20Valid
      (Class|Image|SetBrush Target _slatebrush)
      (return _slatebrush))))